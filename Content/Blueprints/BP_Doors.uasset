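; BP_Doors is a door actor that opens by moving its Door component down when the player character overlaps its Box.
; An IsOpened flag prevents repeat triggering, and BeginPlay or UpdateDoor reapplies the lowered position if already set.
; UpdateDoor is exposed for the level blueprint to work around BeginPlay ordering.
; Opening casts to BP_GameStateBase, but the CallDoorOpened notification to the level blueprint is disconnected.
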(event `UpdateDoor`
  ;[1 1 1] This event calls from the level blueprint by passing the issue with begin play
  ;[1 1 1] Event begin plays are called in random order, too many objects to determine which goes first
  (if (`self.IsOpened?`) :!label _label
    ;[1 1 1] Called when collision happens with the door
    (`SceneComponent.K2_SetRelativeLocation` (`self.Door`) (0.0 0.0 -200.0) false false :!label _label_2)
    (set `self.IsOpened?` true)
    ;;[1 1 1] This calls the binded event on the level blueprint by going through the game state
    (bind _asbp_game_state_base (cast `/Game/Blueprints/SavingLoading/BP_GameStateBase` (`GameplayStatics.GetGameState`)))))

(event `self.ReceiveBeginPlay`
  ;[1 1 1] Event begin plays are called in random order, too many objects to determine which goes first
  (goto _label))

(event `self.Box.OnComponentBeginOverlap`
  (params (OverlappedComponent :type "PrimitiveComponent Object Reference") (OtherActor :type "Actor Object Reference") (OtherComp :type "PrimitiveComponent Object Reference") (OtherBodyIndex :type Integer) (bFromSweep :type Boolean) (SweepResult :type "HitResult Structure (by ref)"))
  ;[1 1 1] Called when collision happens with the door
  (if (and (== OtherActor (`GameplayStatics.GetPlayerCharacter` 0)) (not (`self.IsOpened?`)))
    (goto _label_2)))

(fn `UserConstructionScript`)