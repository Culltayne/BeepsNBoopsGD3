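; BP_Coin2 is a collectible coin that the third-person character picks up by touching it.
; On overlap it adds its own actor reference uniquely to CollectedCoins on the GM_Coding2ForReal game mode's LevelSave, then destroys itself.
; If the save is invalid it only prints a debug message.
; LoadCollectedState, with no caller in this file, marks the coin as collected by swapping its material instead of removing it.
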(event `self.Coin.OnComponentBeginOverlap`
  (params (OverlappedComponent :type "PrimitiveComponent Object Reference") (OtherActor :type "Actor Object Reference") (OtherComp :type "PrimitiveComponent Object Reference") (OtherBodyIndex :type Integer) (bFromSweep :type Boolean) (SweepResult :type "HitResult Structure (by ref)"))
  (cast `/Game/ThirdPerson/Blueprints/BP_ThirdPersonCharacter` OtherActor)
  (bind _asgm_coding_2for_real (cast `/Game/Blueprints/NewSave/GM_Coding2ForReal` (`GameplayStatics.GetGameMode`)))
  (bind _levelsave (`/Game/Blueprints/NewSave/GM_Coding2ForReal.LevelSave` _asgm_coding_2for_real))
  (`/Engine/EditorBlueprintResources/StandardMacros.IsValid` _levelsave
    (:`Is Valid`
      (`KismetArrayLibrary.Array_AddUnique` (`/Game/Blueprints/NewSave/SG_LevelSave.CollectedCoins` _levelsave) self)
      (`self.K2_DestroyActor`))
    (:`Is Not Valid`
      (`KismetSystemLibrary.PrintString` "Failed Unique"))))

(event `LoadCollectedState`
  (`PrimitiveComponent.SetMaterial` (`self.Coin`) 0 "/Game/Footsteps/MI_Tile.MI_Tile")
  (`KismetSystemLibrary.PrintString` "CollectedStateLoaded"))

(fn `UserConstructionScript`)