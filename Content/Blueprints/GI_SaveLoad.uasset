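; Game Instance that saves, loads and deletes player progress and per-level data.
; Init loads or creates the SG_LevelData object for coins to use, stored in a slot named after the current level.
; SavePlayer and LoadPlayer handle stamina and capsule transform through SG_coding2, also triggering the level save or collected-object restore.
; DeleteSaveData clears both slots and reopens the level, without resetting the in-memory LevelData.
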(event `Save Player`
  (bind _slot_name (`self.Slot Name`))
  (`KismetSystemLibrary.PrintString` "Save Player")
  (`self.Save Level`)
  (bind _returnvalue (`GameplayStatics.DoesSaveGameExist` _slot_name)) ; Checks if Exists
  (if _returnvalue
    (bind _returnvalue_2 (`GameplayStatics.LoadGameFromSlot` _slot_name))
    (set `self.PlayerData` _returnvalue_2)
    (else
      (bind _returnvalue_3 (`GameplayStatics.CreateSaveGameObject` "/Game/Blueprints/SG_coding2.SG_coding2_C"))
      (set `self.PlayerData` _returnvalue_3)))
  (bind _assg_coding_2 (cast `/Game/Blueprints/SG_coding2` (`self.PlayerData`)))
  ;[1 1 1] Player Current Data
  (bind _asbp_third_person_character (cast `/Game/ThirdPerson/Blueprints/BP_ThirdPersonCharacter` (`GameplayStatics.GetPlayerCharacter` 0)))
  ;[1 1 1] Save Game Data
  (set `/Game/Blueprints/SG_coding2.PlayerStamina` (`/Game/ThirdPerson/Blueprints/BP_ThirdPersonCharacter.PlayerStamina` _asbp_third_person_character) _assg_coding_2)
  (set `/Game/Blueprints/SG_coding2.PlayerLocation` (`SceneComponent.K2_GetComponentToWorld` (`Character.CapsuleComponent` _asbp_third_person_character)) _assg_coding_2)
  (`GameplayStatics.SaveGameToSlot` _assg_coding_2 _slot_name))

(event `Load Player`
  (bind _slot_name (`self.Slot Name`))
  (`KismetSystemLibrary.PrintString` "Load Player")
  (`self.Load Level`)
  (bind _returnvalue (`GameplayStatics.DoesSaveGameExist` _slot_name))
  (if _returnvalue
    (bind _returnvalue_2 (`GameplayStatics.LoadGameFromSlot` _slot_name))
    (bind _assg_coding_2 (cast `/Game/Blueprints/SG_coding2` _returnvalue_2))
    (bind _asbp_third_person_character (cast `/Game/ThirdPerson/Blueprints/BP_ThirdPersonCharacter` (`GameplayStatics.GetPlayerCharacter` 0)))
    (set `/Game/ThirdPerson/Blueprints/BP_ThirdPersonCharacter.PlayerStamina` (`/Game/Blueprints/SG_coding2.PlayerStamina` _assg_coding_2) _asbp_third_person_character)
    (`SceneComponent.K2_SetWorldTransform` (`Character.CapsuleComponent` _asbp_third_person_character) (`/Game/Blueprints/SG_coding2.PlayerLocation` _assg_coding_2) false false)))

(event `Save Level`
  (`KismetSystemLibrary.PrintString` "Hello")
  (bind _returnvalue (`GameplayStatics.GetCurrentLevelName` true))
  (`GameplayStatics.SaveGameToSlot` (`self.LevelData`) _returnvalue))

(event `Load Level`
  (`KismetSystemLibrary.PrintString` "Level Loaded")
  (bind _returnvalue (`GameplayStatics.GetCurrentLevelName` true))
  (bind _returnvalue_2 (`GameplayStatics.DoesSaveGameExist` _returnvalue))
  (if _returnvalue_2
    (`/Game/Blueprints/SG_LevelData.LoadCollectedObjects` (`self.LevelData`))))

(event `DeleteSaveData`
  (`GameplayStatics.DeleteGameInSlot` (`self.Slot Name`))
  (bind _returnvalue (`GameplayStatics.GetCurrentLevelName` true))
  (`GameplayStatics.DeleteGameInSlot` _returnvalue)
  (if true
    (`KismetSystemLibrary.PrintString` "Deleted Save")
    (bind _returnvalue_2 (`GameplayStatics.GetCurrentLevelName` true))
    (`GameplayStatics.OpenLevel` (`KismetStringLibrary.Conv_StringToName` _returnvalue_2))
    (else
      (`KismetSystemLibrary.PrintString` "Could Not Delete Save"))))

(event `self.ReceiveInit`
  ;[1 0.9375 0] Creating Level Data Variable for coins to talk to
  (bind _returnvalue (`GameplayStatics.GetCurrentLevelName` true))
  (bind _returnvalue_2 (`GameplayStatics.DoesSaveGameExist` _returnvalue))
  (if _returnvalue_2
    (bind _returnvalue_3 (`GameplayStatics.LoadGameFromSlot` _returnvalue))
    (bind _assg_level_data (cast `/Game/Blueprints/SG_LevelData` _returnvalue_3))
    (set `self.LevelData` _assg_level_data)
    (else
      (bind _returnvalue_4 (`GameplayStatics.CreateSaveGameObject` "/Game/Blueprints/SG_LevelData.SG_LevelData_C"))
      (set `self.LevelData` _returnvalue_4))))